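; BP_UiManager is a UI facade that opens the game's store, inventory and skill maker screens and handles a Colosseum entry prompt.
; It caches the player's HUD at BeginPlay and forwards screen, inventory update and interaction key requests to BP_Hud, showing the key hint for Store or SkillMaker tagged targets.
; The message box creates a confirmation widget; confirming shows a loading widget, then a timer opens the battle level.
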(event EventBeginPlay
  (Variables|Default|SetMainHud (HUD|GetHUD (Game|GetPlayerController 0))))

(fn ConstructionScript)

(fn OpenStore
  (params (ItemList :type Array%20of%20ST%20Item%20Structures))
  (bind _asbp_hud (Utilities|Casting|CastToBP_Hud (Variables|Default|GetMainHud)))
  (bind _dointeraction (Default|OpenStoreUi _asbp_hud ItemList))
  (return _dointeraction))

(fn OpenInventory
  (params (ItemData :type Array%20of%20ST%20Item%20Slot%20Structures))
  (bind _asbp_hud (Utilities|Casting|CastToBP_Hud (Variables|Default|GetMainHud)))
  (Default|OpenInventoryUi _asbp_hud ItemData))

(fn UpdateInvetory
  (params (Index :type Integer) (NewItemData :type Array%20of%20ST%20Item%20Slot%20Structures))
  (bind _asbp_hud (Utilities|Casting|CastToBP_Hud (Variables|Default|GetMainHud)))
  (Default|UpdateInventory _asbp_hud Index NewItemData))

(fn OpenSkillMaker
  (params (SkillList :type Array%20of%20ST%20Skill%20Production%20Structures))
  (bind _asbp_hud (Utilities|Casting|CastToBP_Hud (Variables|Default|GetMainHud)))
  (bind _dointeraction (Default|OpenSkillMakerUi _asbp_hud SkillList))
  (return _dointeraction))

(fn OpenMessageBox
  (params (DisplayMessage :type String))
  (bind _returnvalue (Game|GetPlayerController 0))
  ;[0.15 0.15 0.15 0.5] 콜로세움 입장? 위젯 생성
  (bind _returnvalue_2 (UserInterface|CreateWidget "/Game/Blueprints/UI/MoveToBattle/MyRoomWidget.MyRoomWidget_C" (Game|GetPlayerController 0) DisplayMessage))
  (bind _output_get (LocalVariables|SetNewLocalVar _returnvalue_2))
  (EventDispatchers|BindEventtoOnClickedButton _output_get (EventDispatchers|CreateEvent :!event OnButtonClickedEvent))
  (UserInterface|Viewport|AddtoViewport _output_get 0)
  (Input|SetInputModeGameandUI _returnvalue 0 "DoNotLock" false false)
  (Variables|/Script/Engine.PlayerController|SetbShowMouseCursor _returnvalue true)
  (return (LocalVariables|GetNewLocalVar)))

(fn OnButtonClickedEvent
  (params (IsValue :type Boolean))
  (bind _returnvalue (Game|GetPlayerController 0))
  (if IsValue
    ;[0 0 0 0.5] origin script
    (Input|SetInputModeGameOnly _returnvalue false)
    (Variables|/Script/Engine.PlayerController|SetbShowMouseCursor _returnvalue false)
    ;[0.15 0.15 0.15 0.5] loading widget
    (bind _returnvalue_2 (UserInterface|CreateWidget "/Game/Blueprints/UI/Loading/LoadingWIdget.LoadingWIdget_C" 0 3.0))
    (UserInterface|Viewport|AddtoViewport _returnvalue_2 0)
    (Utilities|Time|SetTimerbyFunctionName 0 "OpenLevel" 3.0)))

(fn OpenLevel
  (Game|OpenLevel(byObjectReference) "/Game/Maps/Level_Battle.Level_Battle"))

(fn OpenInteractionUi
  (params (Target :type Actor%20Object%20Reference))
  (bind _asbp_hud (Utilities|Casting|CastToBP_Hud (Variables|Default|GetMainHud)))
  (bind _array_element (Utilities|Array|ForEachLoopwithBreak (Variables|/Script/Engine.Actor|GetTags Target) :!label _label)
    (:LoopBody
      (if (or (== _array_element "Store") (== _array_element "SkillMaker"))
        (Default|UpdateInteractionKeyViewUi _asbp_hud true)
        (goto _label Break)))))

(fn CloseInteractionUi
  (bind _asbp_hud (Utilities|Casting|CastToBP_Hud (Variables|Default|GetMainHud)))
  (Default|UpdateInteractionKeyViewUi _asbp_hud false))