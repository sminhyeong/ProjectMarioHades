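; BP_StoreComponent is an actor component that holds a store's item stock and opens the store UI.
; On BeginPlay it reads every row of its ItemTable data table and appends each found row to ItemList.
; OpenStore casts the game state to BP_GameState, gets its UI manager through OpenUiManager, passes ItemList to that manager's OpenStore and returns the result.
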(event EventBeginPlay
  (CallFunction|StoreDataInitialized (Variables|Default|GetItem%20Table)))

(fn StoreDataInitialized
  (params (ItemTable :type Data%20Table%20Object%20Reference))
  (bind _outrownames (DataTable|GetDataTableRowNames ItemTable))
  (for _array_element _outrownames
    (bind _returnvalue (Utilities|GetDataTableRow ItemTable _array_element)
      (:then
        (Utilities|Array|Add (Variables|Default|GetItemList) _returnvalue)))))

(fn OpenStore
  (bind _asbp_game_state (Utilities|Casting|CastToBP_GameState (Game|GetGameState)))
  (bind _dointeraction (Default|OpenStore (Default|OpenUiManager _asbp_game_state) (Variables|Default|GetItemList)))
  (return _dointeraction))