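; BP_InteractionComponent is an actor component that routes interactions with store and skill maker actors to their UI.
; Interaction uses the passed actor, or falls back to the stored Target, and matches its actor tags to a handler.
; Each handler calls the open function on the target's BP_StoreComponent or BP_SkillMakerComponent.
; The returned DoInteraction state is broadcast through an event dispatcher, and a false result clears Target to end the interaction.
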(event EventBeginPlay)

(event EventTick
  (params (DeltaSeconds :type Float%20%28single-precision%29)))

(fn Interaction
  (params (TargetActor :type Actor%20Object%20Reference))
  ;[0.15 0.15 0.15 0.5] Target Actor가 존재할경우 기존 루틴대로 실행
  ; Target Actor가 존재하지 않을경우 Target이 존재하는지 확인 한 후 기존 루틴대로 실행할지 실행하지 않을지 선택
  (Utilities|IsValid TargetActor
    (:Is%20Valid
      (Variables|Default|SetTarget TargetActor))
    (:Is%20Not%20Valid
      (Utilities|IsValid (Variables|Default|GetTarget)
        (:Is%20Valid
          _))))
  (for _array_element (Variables|/Script/Engine.Actor|GetTags (Variables|Default|GetTarget))
    ;[0.15 0.15 0.15 0.5] 상호작용한 타겟의 Tag를 확인하여 상호작용 함수 실행
    (switch string (Utilities|String|ToString(Name) _array_element)
      (:Store
        (bind _dointeraction (CallFunction|InteractionStore (Variables|Default|GetTarget)))
        (bind _output_get (Variables|Default|SetDoInteraction _dointeraction))
        (Default|CallEventDispatcherDoInteraction _output_get))
      (:SkillMaker
        (bind _dointeraction_2 (CallFunction|InteractionSkillMaker (Variables|Default|GetTarget)))
        (bind _output_get_2 (Variables|Default|SetDoInteraction _dointeraction_2))
        (Default|CallEventDispatcherDoInteraction _output_get_2))))
  ;[0.15 0.15 0.15 0.5] 상호작용함수들의 리턴값을 통해 상호작용이 종료됐나 확인하여 Target을 NULL로 초기화
  (if (not (Variables|Default|GetDoInteraction))
    (Variables|Default|SetTarget 0)))

(fn InteractionStore
  (params (Target :type Actor%20Object%20Reference))
  (bind _returnvalue (Actor|GetComponentbyClass Target "/Game/SMH/Components/BP_StoreComponent.BP_StoreComponent_C"))
  (Utilities|IsValid _returnvalue
    (:Is%20Valid
      (bind _dointeraction (Default|OpenStore _returnvalue))
      (return _dointeraction))))

(fn InteractionSkillMaker
  (params (Target :type Actor%20Object%20Reference))
  (bind _returnvalue (Actor|GetComponentbyClass Target "/Game/SMH/Components/BP_SkillMakerComponent.BP_SkillMakerComponent_C"))
  (Utilities|IsValid _returnvalue
    (:Is%20Valid
      (bind _dointeraction (Default|OpenSkillMakerUi _returnvalue))
      (return _dointeraction))))