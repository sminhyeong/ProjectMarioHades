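; BP_SkillMakerComponent is an actor component that supplies skill production data to the Skill Maker UI.
; On BeginPlay it loops over SkillTable row names, merging production, skill and material rows from three data tables into SkillList.
; The material lookup uses the production row's MaterialRowName, and entries are added only when that lookup succeeds.
; OpenSkillMakerUi passes the cached list to the UI manager obtained from BP_GameState.
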(event EventBeginPlay
  (CallFunction|SetSkillMaker))

(fn SetSkillMaker
  (bind _outrownames (DataTable|GetDataTableRowNames (Variables|Default|GetSkillTable)))
  (for _array_element _outrownames
    (Utilities|FlowControl|Sequence
      (:then_0
        (bind _returnvalue (Utilities|GetDataTableRow "/Game/SMH/SkillMaker/DT_SkillPRoduction.DT_SkillPRoduction" _array_element)
          (:then
            (bind _output_get (LocalVariables|SetTempSkill _returnvalue))
            (Utilities|Struct|SetmembersinST_SkillProduction _output_get _array_element))))
      (:then_1
        (bind _returnvalue_2 (Utilities|GetDataTableRow "/Game/Skills/DT_Skill.DT_Skill" _array_element)
          (:then
            (Utilities|Struct|SetmembersinST_SkillProduction (LocalVariables|GetTempSkill) _returnvalue_2))))
      (:then_2
        (bind _returnvalue_3 (Utilities|GetDataTableRow "/Game/Items/DT_MaterialItem.DT_MaterialItem" (.materialrowname (LocalVariables|GetTempSkill)))
          (:then
            (bind _structout (Utilities|Struct|SetmembersinST_SkillProduction (LocalVariables|GetTempSkill) _returnvalue_3))
            (Utilities|Array|Add (Variables|Default|GetSkillList) _structout)))))))

(fn OpenSkillMakerUi
  (bind _asbp_game_state (Utilities|Casting|CastToBP_GameState (Game|GetGameState)))
  (bind _dointeraction (Default|OpenSkillMaker (Default|OpenUiManager _asbp_game_state) (Variables|Default|GetSkillList)))
  (return _dointeraction))