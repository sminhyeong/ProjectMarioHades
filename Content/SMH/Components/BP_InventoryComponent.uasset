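; Inventory component that stores item slots, each pairing item data with a count, and passes them to the game state's UI manager for display.
; Adding stacks by item name up to a 999 cap, then starts a new slot.
; Removing decrements a slot or deletes it when emptied, and a count query totals matching slots.
; BeginPlay seeds the inventory with random DT_Item rows through a test function.
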(event EventBeginPlay
  (CallFunction|TestAddItem))

(fn AddItem
  (params (NewItem :type ST%20Item%20Structure))
  (bind (_array_element _array_index) (Utilities|Array|ForEachLoopwithBreak (Variables|Default|GetItems) :!label _label)
    (:LoopBody
      (bind _output_get (LocalVariables|SetCurrentItem _array_element))
      (if (CallFunction|IsExistItem (.itemdata _output_get) NewItem)
        (if (not (CallFunction|IsFullCount (LocalVariables|GetCurrentItem)))
          (LocalVariables|SetIsExist true)
          (LocalVariables|SetCurIndex _array_index)
          (goto _label Break))))
    (:Completed
      (if (LocalVariables|GetIsExist)
        (Math|Integer|IncrementInt (.Count (Utilities|Struct|BreakST_ItemSlot (Utilities|Array|Get(acopy) (Variables|Default|GetItems) (LocalVariables|GetCurIndex)))))
        (else
          (bind _output_get_2 (LocalVariables|SetCurrentItem (Utilities|Struct|MakeST_ItemSlot 1 NewItem)))
          (Utilities|Array|Add (Variables|Default|GetItems) _output_get_2))))))

(fn ReMoveItem
  (params (Index :type Integer) (Count :type Integer))
  (bind _items (Variables|Default|GetItems))
  (bind _output (Utilities|Array|Get(acopy) _items Index))
  (bind _count (Utilities|Struct|BreakST_ItemSlot _output))
  (bind _returnvalue (- _count Count))
  (if (<= _returnvalue 0)
    (Utilities|Array|RemoveIndex (Variables|Default|GetItems) Index)
    (else
      (Utilities|Struct|SetmembersinST_ItemSlot _output _returnvalue))))

(fn IsExistItem
  (params (CurItem :type ST%20Item%20Structure) (ST_Item :type ST%20Item%20Structure%20%28by%20ref%29))
  (return (Utilities|Enum|Equal(Enum) (.Name (Utilities|Struct|BreakST_Item CurItem)) (.Name (Utilities|Struct|BreakST_Item ST_Item)))))

(fn IsFullCount
  (params (ST_Item :type ST%20Item%20Slot%20Structure%20%28by%20ref%29))
  (return (> (+ (.count ST_Item) 1) 999)))

(fn TestAddItem
  (for _index (range 0 5)
    (bind _outrownames (DataTable|GetDataTableRowNames "/Game/Items/DT_Item.DT_Item"))
    (bind _returnvalue (Utilities|GetDataTableRow "/Game/Items/DT_Item.DT_Item" (.OutItem (Utilities|Array|Random _outrownames)))
      (:then
        (CallFunction|AddItem _returnvalue)))))

(fn OpenInventory
  (bind _asbp_game_state (Utilities|Casting|CastToBP_GameState (Game|GetGameState)))
  (Default|OpenInventory (Default|OpenUiManager _asbp_game_state) (Variables|Default|GetItems)))

(fn GetItemCount
  (params (ItemName :type String))
  (for _array_element (Variables|Default|GetItems)
    (if (Utilities|Enum|Equal(Enum) (.name (.ItemData (Utilities|Struct|BreakST_ItemSlot _array_element))) ItemName)
      (LocalVariables|SetTempCount (+ (.Count (Utilities|Struct|BreakST_ItemSlot _array_element)) (LocalVariables|GetTempCount)))))
  (return (LocalVariables|GetTempCount)))