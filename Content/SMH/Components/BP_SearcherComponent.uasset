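; Searcher component that picks its owner's current target from registered actors and broadcasts target changes.
; AddTarget starts a looping FindTarget timer that selects the nearest actor, optionally pre-filtered by a dot-product view-angle check.
; The view check subtracts the owner's forward vector, not its location, from the target position.
; Removals are queued until after each search; an empty list stops the timer and broadcasts RemoveTarget.
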(event EventBeginPlay)

(event EventTick
  (params (DeltaSeconds :type Float%20%28single-precision%29)))

(fn AddTarget
  (params (SearchItem :type Actor%20Object%20Reference))
  (Utilities|Array|Add (Variables|Default|GetTargets) SearchItem)
  (if (not (Class|KismetSystemLibrary|IsTimerActive 0 "FindTarget"))
    (Utilities|Time|SetTimerbyFunctionName 0 "FindTarget" 0.1 true)
    (Development|PrintString "StartFilter")))

(fn RemoveTarget
  (params (Target :type Actor%20Object%20Reference))
  (Utilities|Array|Add (Variables|Default|GetRemoveTargetList) Target))

(fn FindTarget
  (switch Utilities|FlowControl|Switch|SwitchonEN_FindMode (Variables|Default|GetFindMode)
    (:NewEnumerator1
      (CallFunction|FindeNearestTarget (Variables|Default|GetTargets)))
    (:NewEnumerator3
      (CallFunction|FindNearestandViewSightTarget)))
  (CallFunction|RemoveList))

(fn FindeNearestTarget
  (params (ActorsToCheck :type Array%20of%20Actor%20Object%20References))
  (bind _returnvalue (Components|GetOwner))
  (bind _returnvalue_2 (Transformation|GetActorLocation _returnvalue))
  (bind _returnvalue_3 (Actor|FindNearestActor _returnvalue_2 ActorsToCheck))
  (bind _targetactor (Variables|Default|GetTargetActor)
    (:then
      (if (!= _targetactor _returnvalue_3)
        (bind _output_get (Variables|Default|SetTargetActor _returnvalue_3))
        (Default|CallEventDispatcherTargetUpdate _output_get)))
    (:else
      (bind _output_get_2 (Variables|Default|SetTargetActor _returnvalue_3))
      (Default|CallEventDispatcherTargetUpdate _output_get_2))))

(fn FindNearestandViewSightTarget
  (for _array_element (Variables|Default|GetTargets)
    (if (CallFunction|IsinFieldOfView _array_element)
      (Utilities|Array|Add (LocalVariables|GetTempTargets) _array_element)))
  (CallFunction|FindeNearestTarget (LocalVariables|GetTempTargets)))

(fn GetTarget
  (return (Variables|Default|GetTargetActor)))

(fn RemoveList
  (bind _removetargetlist (Variables|Default|GetRemoveTargetList))
  (for _array_element _removetargetlist
    (Utilities|Array|RemoveItem (Variables|Default|GetTargets) _array_element))
  (Utilities|Array|Clear _removetargetlist)
  (if (Utilities|Array|IsEmpty (Variables|Default|GetTargets))
    (Utilities|Time|ClearTimerbyFunctionName 0 "FindTarget")
    (Variables|Default|SetTargetActor 0)
    (Default|CallEventDispatcherRemoveTarget)))

(fn IsinFieldOfView
  (params (self2 :type Actor%20Object%20Reference))
  (return (>= (Math|Vector|DotProduct (Transformation|GetActorForwardVector (Components|GetOwner)) (Math|Vector|Normalize (- (Transformation|GetActorLocation self2) (Transformation|GetActorForwardVector (Components|GetOwner))))) (Math|Trig|Cos(Degrees) (Variables|Default|GetViewAngle)))))