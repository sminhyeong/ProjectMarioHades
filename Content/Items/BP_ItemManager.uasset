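; BP_ItemManager applies item effects to the monster that owns it.
; UseItem switches on item type; for Change HP it casts the owner to BP_MonsterBase and passes its BP_CharStateComp character state to HealItem.
; HealItem adds HealHP to current HP, clamped between zero and max HP.
; SKillItem is an empty stub, and BeginPlay and Tick are unused.
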(event EventBeginPlay)

(event EventTick
  (params (DeltaSeconds :type Float%20%28single-precision%29)))

(fn UseItem
  (params (ItemType :type EN_ItemType%20Enum :default "NewEnumerator0"))
  (switch Utilities|FlowControl|Switch|SwitchonEN_ItemType ItemType
    (:NewEnumerator0
      (bind _asbp_monster_base (Utilities|Casting|CastToBP_MonsterBase (Components|GetOwner)))
      (CallFunction|HealItem (Variables|/Game/Class/Common/BP_CharStateComp.BP_CharStateComp_C|GetCurCharstate (Actor|GetComponentbyClass _asbp_monster_base "/Game/Class/Common/BP_CharStateComp.BP_CharStateComp_C"))))))

(fn HealItem
  (params (CharState :type ST%20Cur%20Charstate%20Structure%20%28by%20ref%29))
  (bind (_chardata _curhp) (Utilities|Struct|BreakST_CurCharstate CharState))
  (Utilities|Struct|SetmembersinST_CurCharstate CharState (Math|Float|Clamp(Float) (+ _curhp (Variables|Default|GetHealHP)) 0.0 (.maxhp _chardata))))

(fn SKillItem)