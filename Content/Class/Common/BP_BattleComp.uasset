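; Battle component that tracks a character's current HP through damage and healing, both ignored when the caller flags the character as dead.
; GetDamage and GetHeal modify the CurCharstate struct and broadcast DSUpdateHP with max and current HP for listeners.
; GetDamage broadcasts DSDeath when HP reaches zero or below.
; GetHeal caps HP at MaxHp only after broadcasting, so listeners can receive an over-max value.
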(event EventBeginPlay)

(event EventTick
  (params (DeltaSeconds :type Float%20%28single-precision%29)))

(fn GetDamage
  (params (DamageGet :type Float%20%28double-precision%29) (isdead :type Boolean))
  (bind _curcharstate (Variables|Default|GetCurCharstate))
  ;[0.15 0.15 0.15 0.5] 받은 데미지 현재 체력에 저장, 예외-죽음
  (if (not isdead)
    (bind _structout (Utilities|Struct|SetmembersinST_CurCharstate (Variables|Default|GetCurCharstate) (- (.curhp (Variables|Default|GetCurCharstate)) DamageGet)))
    (Default|CallDSUpdateHP (.maxhp (.chardata _curcharstate)) (.curhp _curcharstate))
    ;[0.15 0.15 0.15 0.5] 캐릭터 사망여부
    (if (<= (.CurHp (Utilities|Struct|BreakST_CurCharstate _structout)) 0.0)
      (Default|CallDSDeath true))))

(fn GetHeal
  (params (Heal :type Float%20%28double-precision%29) (isDead :type Boolean))
  ;[0.15 0.15 0.15 0.5] 받은 체력 저장/ 예외 죽음
  (if (not isDead)
    (bind _structout (Utilities|Struct|SetmembersinST_CurCharstate (Variables|Default|GetCurCharstate) (+ (.curhp (Variables|Default|GetCurCharstate)) Heal)))
    (Default|CallDSUpdateHP (.maxhp (.chardata (Variables|Default|GetCurCharstate))) (.curhp (Variables|Default|GetCurCharstate)))
    ;[0.15 0.15 0.15 0.5] 체력 최대 이상 회복시 최대로 맞추기
    (if (>= (.CurHp (Utilities|Struct|BreakST_CurCharstate _structout)) (.maxhp (.CharData (Utilities|Struct|BreakST_CurCharstate _structout))))
      (Variables|Default|SetCurCharstate (Utilities|Struct|MakeST_CurCharstate "(Name_11_64B7035D4C848B674387C6848081152E=\"\",ClassType_13_143597744210D746785D8B94B64C8951=None,MaxHp_9_CF1EDDBA47A47413FA37178D1D8EA950=0.000000)" (.maxhp (.CharData (Utilities|Struct|BreakST_CurCharstate _structout))))))))