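; BP_WidgetComp is a component that gives its owning actor an HP widget.
; On BeginPlay it creates WID_HPWidget, passes itself in and adds it to the viewport as a screen widget, then removes it on EndPlay.
; BindSocket returns the location of the HP_Socket socket on the owner's StaticMeshComponent, providing an anchor point for the widget.
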(event EventBeginPlay
  (CallFunction|Createwidget))

(event EventEndPlay
  (params (EndPlayReason :type EEndPlayReason%20Enum :default "Destroyed"))
  (Widget|RemovefromParent (Variables|Default|GetHPwidget)))

(fn Createwidget
  (bind _returnvalue (UserInterface|CreateWidget "/Game/Class/Common/WID_HPWidget.WID_HPWidget_C" 0 self))
  (bind _output_get (Variables|Default|SetHPwidget _returnvalue))
  (UserInterface|Viewport|AddtoViewport _output_get 0))

(fn BindSocket
  (return (Transformation|GetSocketLocation (Actor|GetComponentbyClass (Components|GetOwner) "/Script/Engine.StaticMeshComponent") "HP_Socket")))