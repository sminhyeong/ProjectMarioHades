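; BP_TestObject is a sandbag dummy for combat testing that hurts overlapping actors and takes damage itself.
; On BeginPlay it sets BP_CharStateComp to "Dummy" and binds an HP-update event on BP_BattleComp.
; Incoming damage goes to BP_BattleComp, and the HP update handler prints max and current HP.
; Socket capsule-trace and DT_Skill-driven attack functions exist but are not called in this graph.
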(event Game|Damage|EventAnyDamage
  (params (Damage :type Float%20%28single-precision%29) (DamageType :type Damage%20Type%20Object%20Reference) (InstigatedBy :type Controller%20Object%20Reference) (DamageCauser :type Actor%20Object%20Reference))
  ;[0.15 0.15 0.15 0.5] 데미지 받음
  (Default|GetDamage (Actor|GetComponentbyClass "/Game/Class/Common/BP_BattleComp.BP_BattleComp_C") Damage false))

(event EventBeginPlay
  ;[0.15 0.15 0.15 0.5] 초기설정 및 위젯에 업데이트
  (CallFunction|BindState))

(event Collision|EventActorBeginOverlap
  (params (OtherActor :type Actor%20Object%20Reference))
  ;[0.15 0.15 0.15 0.5] 데미지 줌
  (Game|Damage|ApplyDamage (Variables|Default|GetActor) 1e+01 0 self))

(fn ConstructionScript)

(fn EVUpdateStatetoWidget
  (params (MaxHP :type Float%20%28double-precision%29) (CurHP :type Float%20%28double-precision%29))
  (Development|PrintString (Utilities|String|Append "SandBack" ":" "MaxHp" ":" (Utilities|String|ToString(Float) MaxHP) "CurHp" ":" (Utilities|String|ToString(Float) CurHP))))

(fn BindState
  (Default|SetCharState (Actor|GetComponentbyClass "/Game/Class/Common/BP_CharStateComp.BP_CharStateComp_C") "Dummy")
  (EventDispatchers|BindEventtoDSUpdateHP (Actor|GetComponentbyClass "/Game/Class/Common/BP_BattleComp.BP_BattleComp_C") (EventDispatchers|CreateEvent :!event EVUpdateStatetoWidget)))

(fn AttackOverLapCheck
  ;[0.15 0.15 0.15 0.5] 소켓 위치
  (bind _output_get (LocalVariables|SetNewLocalVar (Transformation|GetSocketLocation (Variables|/Script/Engine.Actor|GetRootComponent (Variables|Default|GetActor)) (LocalVariables|GetSocketName))))
  ;[0.15 0.15 0.15 0.5] 트레이스 오브젝트-
  ; 1.충돌된 오브젝트들 멀티 체크
  ; 2. 오브젝트 내보내기
  (bind _outhits (Class|KismetSystemLibrary|CapsuleTraceMultiforObjects _output_get _output_get 15.0 1e+01 (Utilities|Array|MakeArray "ObjectTypeQuery1" "ObjectTypeQuery2" "ObjectTypeQuery3" "ObjectTypeQuery4") false 0 "None" true))
  (for _array_element _outhits
    (return (.HitActor (Collision|BreakHitResult _array_element)))))

(fn DoDamage
  (params (Onhit :type Actor%20Object%20Reference))
  ;[0.15 0.15 0.15 0.5] 사용할 스킬 데이터(이름)
  (bind _returnvalue (Utilities|GetDataTableRow "/Game/Skills/DT_Skill.DT_Skill" (Variables|Default|GetRow%20Name))
    (:then
      ;[0.15 0.15 0.15 0.5] 스킬매니저- 애니메이션 처리
      ; *스킬매니저 장착필요
      (Default|DoUseSkill (Actor|GetComponentbyClass "/Game/Skills/BP_SkillManager.BP_SkillManager_C") _returnvalue)
      ;[0.15 0.15 0.15 0.5] 데미지 처리
      (Game|Damage|ApplyDamage 0 (.Damage (Utilities|Struct|BreakST_Skill _returnvalue)) (Pawn|GetController (Variables|Default|GetCharacter)) self)
      (return 0))))