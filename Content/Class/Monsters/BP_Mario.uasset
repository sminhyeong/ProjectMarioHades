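; BP_Mario is an input-driven character Blueprint under Monsters that adds targeted interaction and inventory access to its parent class.
; A collision volume feeds overlapping actors, excluding itself, into the searcher component, whose current target is passed to the interaction component on the interact input.
; The inventory input opens the inventory component only while no interaction is active, and BeginPlay binds to the interaction dispatcher.
; DoDamage is an empty stub.
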(event Input|EnhancedActionEvents|EnhancedInputActionIA_Interaction
  (params (ActionValue :type Vector%202D%20Structure) (ElapsedSeconds :type Float%20%28double-precision%29) (TriggeredSeconds :type Float%20%28double-precision%29) (InputAction :type Input%20Action%20Object%20Reference :default "/Game/ThirdPerson/Input/Actions/IA_Interaction.IA_Interaction"))
  (:Started
    (Default|Interaction (Variables|Default|GetBP_InteractionComponent) (Default|GetTarget (Variables|Default|GetBP_SearcherComponent)))))

(event Input|EnhancedActionEvents|EnhancedInputActionIA_Inventory
  (params (ActionValue :type Boolean) (ElapsedSeconds :type Float%20%28double-precision%29) (TriggeredSeconds :type Float%20%28double-precision%29) (InputAction :type Input%20Action%20Object%20Reference :default "/Game/ThirdPerson/Input/Actions/IA_Inventory.IA_Inventory"))
  (:Started
    (if (not (Variables|/Game/SMH/Components/BP_InteractionComponent.BP_InteractionComponent_C|GetDoInteraction (Variables|Default|GetBP_InteractionComponent)))
      (Default|OpenInventory (Variables|Default|GetBP_InventoryComponent)))))

(event EventBeginPlay
  (|CallParentFunction)
  (EventDispatchers|BindEventtoEventDispatcherDoInteraction (Variables|Default|GetBP_InteractionComponent) (EventDispatchers|CreateEvent :!event EventDoInteraction)))

(event OnComponentBeginOverlap(SearcherColision)
  (params (OverlappedComponent :type Primitive%20Component%20Object%20Reference) (OtherActor :type Actor%20Object%20Reference) (OtherComp :type Primitive%20Component%20Object%20Reference) (OtherBodyIndex :type Integer) (bFromSweep :type Boolean) (SweepResult :type Hit%20Result%20Structure%20%28by%20ref%29))
  (if (!= OtherActor self)
    (Default|AddTarget (Variables|Default|GetBP_SearcherComponent) OtherActor)))

(event OnComponentEndOverlap(SearcherColision)
  (params (OverlappedComponent :type Primitive%20Component%20Object%20Reference) (OtherActor :type Actor%20Object%20Reference) (OtherComp :type Primitive%20Component%20Object%20Reference) (OtherBodyIndex :type Integer))
  (if (!= OtherActor self)
    (Default|RemoveTarget (Variables|Default|GetBP_SearcherComponent) OtherActor)))

(fn ConstructionScript
  (|CallParentFunction))

(fn DoDamage
  (params (Onhit :type Actor%20Object%20Reference) (SkillUse :type Name :default "None"))
  (return 0))