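; Monster state component that tracks a monster's current stats and health and handles damage.
; SetMonState looks up a named row in DT_MonState, initializes the current state at max HP and broadcasts the update.
; GetDamage ignores monsters already dead, otherwise subtracts HP without clamping and broadcasts the new value.
; A death dispatcher fires with the state when HP drops to zero or below.
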(event EventBeginPlay)

(event EventTick
  (params (DeltaSeconds :type Float%20%28single-precision%29)))

(fn GetDamage
  (params (Damage :type Float%20%28double-precision%29))
  (bind _curmonstate (Variables|Default|GetCurMonstate))
  (if (not (CallFunction|IsDead))
    (bind _structout (Utilities|Struct|SetmembersinST_CurMonstate (Variables|Default|GetCurMonstate) (- (.curhp (Variables|Default|GetCurMonstate)) Damage)))
    (Default|CallDSUpdateHp (.curhp _curmonstate) (.maxhp (.mondata _curmonstate)))
    (if (<= (.CurHp (Utilities|Struct|BreakST_CurMonstate _structout)) 0.0)
      (Default|CallDSDeath (Variables|Default|GetCurMonstate)))))

(fn IsDead
  (return (<= (.curhp (Variables|Default|GetCurMonstate)) 0.0)))

(fn SetMonState
  (params (Name :type Name))
  (bind _returnvalue (Utilities|GetDataTableRow "/Game/Class/Monsters/AI/DT_MonState.DT_MonState" Name)
    (:then
      (bind _output_get (Variables|Default|SetCurMonstate (Utilities|Struct|MakeST_CurMonstate "(Name_11_64B7035D4C848B674387C6848081152E=\"\",Monstertype_6_143597744210D746785D8B94B64C8951=None,MaxHp_9_CF1EDDBA47A47413FA37178D1D8EA950=0.000000)" (.MaxHp (Utilities|Struct|BreakST_Monstate _returnvalue)))))
      (Default|CallDSUpdateMonState _output_get))))