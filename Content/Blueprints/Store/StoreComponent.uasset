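; StoreComponent is a Blueprint component that creates the in-game store UI and adds it to the viewport on BeginPlay.
; It builds one item slot widget per DT_Item data table row, passing the row data and index, and adds each to the StoreBorder widget.
; Each slot's buy-click dispatcher is bound to an event.
; BuyItem is a stub that only prints item name and slot index.
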(event EventBeginPlay
  (bind _returnvalue (UserInterface|CreateWidget "/Game/Blueprints/UI/Store/StoreBorder.StoreBorder_C"))
  (bind _output_get (Variables|Default|SetStoreBorder _returnvalue))
  (CallFunction|StoreInitialized)
  (UserInterface|Viewport|AddtoViewport _output_get 0))

(fn StoreInitialized
  (bind _outrownames (DataTable|GetDataTableRowNames "/Game/Items/DT_Item.DT_Item"))
  (for (_array_element _array_index) _outrownames
    (bind _returnvalue (Utilities|GetDataTableRow "/Game/Items/DT_Item.DT_Item" _array_element)
      (:then
        (bind _returnvalue_2 (UserInterface|CreateWidget "/Game/Blueprints/UI/Store/StoreItemSlotWidget.StoreItemSlotWidget_C" 0 _returnvalue _array_index))
        (EventDispatchers|BindEventtoEventDispatcheronClickedBuy _returnvalue_2 (EventDispatchers|CreateEvent :!event BuyItem))
        (Default|AddItemSlot (Variables|Default|GetStoreBorder) _returnvalue_2)))))

(fn BuyItem
  (params (ItemData :type ST%20Item%20Structure) (SlotIndex :type Integer))
  (Development|PrintString (Utilities|String|Append "Item Name ; " (.name ItemData) ", Slot Idx : " (Utilities|String|ToString(Integer) SlotIndex))))