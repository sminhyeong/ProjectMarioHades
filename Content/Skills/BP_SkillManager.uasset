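; Skill manager component that holds its owner's skills and plays their attacks.
; AddSkill loads rows from DT_Skill; IsExistSkill looks skills up by type.
; Tick advances each skill's cooldown timer, wrapping it to zero past CoolTime, without triggering or gating use.
; DoUseSkill checks CanAttack, plays the owner Character's montage, broadcasts damage via dispatcher and re-enables attacking on a timer set to montage length.
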(event EventBeginPlay)

(event EventTick
  (params (DeltaSeconds :type Float%20%28single-precision%29))
  (CallFunction|UpdateSkill DeltaSeconds))

(fn AddSkill
  (params (SkillRowName :type Name))
  ;[0.15 0.15 0.15 0.5] 배열에 스킬 추가
  (bind _returnvalue (Utilities|GetDataTableRow "/Game/Skills/DT_Skill.DT_Skill" SkillRowName)
    (:then
      (Utilities|Array|Add (Variables|Default|GetSkills) (Utilities|Struct|MakeST_CurSkil _returnvalue (.CoolTime (Utilities|Struct|BreakST_Skill _returnvalue))))
      (Development|PrintString (Utilities|String|Append "Add Skill : " (.Name (Utilities|Struct|BreakST_Skill _returnvalue))) true true "(R=1.000000,G=0.000000,B=0.717914,A=1.000000)" 5.0))
    (:RowNotFound
      (Development|PrintString "asasdsadHello"))))

(fn UpdateSkill
  (params (DeltaSecond :type Float%20%28double-precision%29))
  ;[0.15 0.15 0.15 0.5] 쿨타임 업데이트
  (for (_ _array_index) (Variables|Default|GetSkills)
    (CallFunction|UpdateSkillCoolTime (Utilities|Array|Get(acopy) (Variables|Default|GetSkills) _array_index) DeltaSecond)))

(fn DoUseSkill
  (params (SkilltoUse :type ST%20Skill%20Structure))
  (bind (_name _skilltype _skillanimation _skillusetime _cooltime _damage) (Utilities|Struct|BreakST_Skill SkilltoUse))
  ;[0.15 0.15 0.15 0.5] 로그 출력
  ;;[0.15 0.15 0.15 0.5] Comment
  (if (Variables|Default|GetCanAttack)
    (Variables|Default|SetCanAttack false)
    (Development|PrintString (Utilities|String|Append "Use Skill : " _name))
    ;[0.15 0.15 0.15 0.5] 애니메이션 출력
    (bind _ascharacter (Utilities|Casting|CastToCharacter (Components|GetOwner)))
    (bind _returnvalue (Animation|PlayAnimMontage _ascharacter _skillanimation _skillusetime "None"))
    (Utilities|Time|SetTimerbyFunctionName 0 "EndAttackAnim" _returnvalue)
    (Default|CallDSDoUseSkill _damage)))

(fn UpdateSkillCoolTime
  (params (CurSkill :type ST%20Cur%20Skil%20Structure%20%28by%20ref%29) (DeltaSecond :type Float%20%28double-precision%29))
  ;[0.15 0.15 0.15 0.5] 쿨 계산
  (bind _structout (Utilities|Struct|SetmembersinST_CurSkil CurSkill (+ (.CurCoolTime (Utilities|Struct|BreakST_CurSkil CurSkill)) DeltaSecond)))
  (if (> (.CurCoolTime (Utilities|Struct|BreakST_CurSkil _structout)) (.cooltime (.SkillData (Utilities|Struct|BreakST_CurSkil _structout))))
    ;[0.15 0.15 0.15 0.5] 쿨타임 초기화
    (Utilities|Struct|SetmembersinST_CurSkil _structout 0.0)))

(fn EVSendTarget
  (params (OverlappedActor :type Actor%20Object%20Reference)))

(fn IsExistSkill
  (params (SkillType :type EN_SkillType%20Enum :default "NewEnumerator0"))
  (for _array_element (Variables|Default|GetSkills)
    (Development|PrintString (.Name (Utilities|Struct|BreakST_Skill (.SkillData (Utilities|Struct|BreakST_CurSkil _array_element)))) true true "(R=0.000000,G=0.660000,B=1.000000,A=1.000000)" 4.0)
    (if (Utilities|Enum|Equal(Enum) (.SkillType (Utilities|Struct|BreakST_Skill (.SkillData (Utilities|Struct|BreakST_CurSkil _array_element)))) SkillType)
      (return true)))
  (return false))

(fn EndAttackAnim
  (Variables|Default|SetCanAttack true))