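; BP_SkillBase is a base skill actor that deals damage when its sphere begins overlapping, then destroys itself.
; On overlap it runs a capsule trace at its own location, ignoring the player character, with debug drawing and a printout of the first hit.
; The trace check feeds DoDamage, which looks up the hard-coded "fireball" row in DT_Skill and applies that damage with the player controller as instigator.
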(event OnComponentBeginOverlap(Sphere)
  (params (OverlappedComponent :type Primitive%20Component%20Object%20Reference) (OtherActor :type Actor%20Object%20Reference) (OtherComp :type Primitive%20Component%20Object%20Reference) (OtherBodyIndex :type Integer) (bFromSweep :type Boolean) (SweepResult :type Hit%20Result%20Structure%20%28by%20ref%29))
  (CallFunction|SkillDMG))

(event EventBeginPlay)

(event Collision|EventActorBeginOverlap
  (params (OtherActor :type Actor%20Object%20Reference)))

(event EventTick
  (params (DeltaSeconds :type Float%20%28single-precision%29)))

(fn ConstructionScript)

(fn SkillDMG
  (bind _onhitactor (CallFunction|AttackOverLapCheck))
  (CallFunction|DoDamage _onhitactor "fireball")
  (Actor|DestroyActor))

(fn AttackOverLapCheck
  ;[0.15 0.15 0.15 0.5] 소켓 위치
  (bind _output_get (Variables|Default|SetSocketLoc (Transformation|GetActorLocation)))
  ;[0.15 0.15 0.15 0.5] 트레이스 오브젝트-
  ; 1.충돌된 오브젝트들 멀티 체크
  ; 2. 오브젝트 내보내기
  (Rendering|Debug|DrawDebugCapsule _output_get 15.0 15.0 "0, 0, 0" "(R=1.000000,G=0.000000,B=0.504485,A=1.000000)" 3.0 3.0)
  (bind _outhits (Class|KismetSystemLibrary|CapsuleTraceMultiforObjects _output_get _output_get 15.0 1e+01 (Utilities|Array|MakeArray "ObjectTypeQuery1" "ObjectTypeQuery2" "ObjectTypeQuery3" "ObjectTypeQuery4") false (Utilities|Array|MakeArray (Game|GetPlayerCharacter 0)) "None" true))
  (for _array_element _outhits
    (Development|PrintString (Utilities|String|Append "OnHitIs" (Utilities|GetDisplayName (.HitActor (Collision|BreakHitResult _array_element)))))
    (return 0)))

(fn DoDamage
  (params (Onhit :type Actor%20Object%20Reference) (SkillUse :type Name :default "None"))
  ;[0.15 0.15 0.15 0.5] 사용할 스킬 데이터(이름)
  (bind _returnvalue (Utilities|GetDataTableRow "/Game/Skills/DT_Skill.DT_Skill" SkillUse)
    (:then
      ;[0.15 0.15 0.15 0.5] 데미지 처리
      (Game|Damage|ApplyDamage Onhit (.Damage (Utilities|Struct|BreakST_Skill _returnvalue)) (Game|GetPlayerController 0) self)
      (return 0))))