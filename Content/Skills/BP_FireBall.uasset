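; BP_FireBall is a fireball skill projectile that moves along its forward vector at Speed and expires after three seconds via life span.
; Tick offsets the Sphere component without sweep, and Sphere overlap calls SkillDMG, which defers to the parent implementation.
; DoDamage is empty, and the older timer-to-StopSkill destruction and radial damage nodes are left disconnected.
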(event OnComponentBeginOverlap(Sphere)
  (params (OverlappedComponent :type Primitive%20Component%20Object%20Reference) (OtherActor :type Actor%20Object%20Reference) (OtherComp :type Primitive%20Component%20Object%20Reference) (OtherBodyIndex :type Integer) (bFromSweep :type Boolean) (SweepResult :type Hit%20Result%20Structure%20%28by%20ref%29))
  (CallFunction|SkillDMG))

(event EventBeginPlay
  (|CallParentFunction)
  ;[0.15 0.15 0.15 0.5] 이게 더 간편해보여서 수정
  (Actor|SetLifeSpan 3.0))

(event EventTick
  (params (DeltaSeconds :type Float%20%28single-precision%29))
  (|CallParentFunction DeltaSeconds)
  (Transformation|AddWorldOffset (Variables|Default|GetSphere) (* (Transformation|GetActorForwardVector) (* DeltaSeconds (Variables|Default|GetSpeed))) false false))

(fn ConstructionScript
  (|CallParentFunction))

(fn StopSkill
  (Actor|DestroyActor))

(fn DoDamage
  (params (Onhit :type Actor%20Object%20Reference) (SkillUse :type Name :default "None"))
  (return 0))

(fn SkillDMG
  (|CallParentFunction))