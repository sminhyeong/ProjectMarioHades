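; BP_WeaponBase is a base weapon Blueprint that a character carries and triggers.
; EventAttachToChar stores the character and snaps the weapon to its mesh without a socket, while EventDetachFromChar detaches it at its world transform and clears that reference.
; A press in EventTrigger calls DoTrigger, which plays a montage on a valid character, though no animation exists yet.
; BeginPlay, overlap, Tick and the construction script are empty.
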(event EventBeginPlay)

(event Collision|EventActorBeginOverlap
  (params (OtherActor :type Actor%20Object%20Reference)))

(event EventTick
  (params (DeltaSeconds :type Float%20%28single-precision%29)))

(fn ConstructionScript)

(fn DoTrigger
  (bind _character (Variables|Default|GetCharacter)
    (:then
      ;[0.15 0.15 0.15 0.5] 애니메이션 안만들었음!
      (Animation|PlayAnimMontage _character 0 1.0 "None"))
    (:else)))

(fn EventAttachtoChar
  (params (Character :type Character%20Object%20Reference))
  (bind _output_get (Variables|Default|SetCharacter Character))
  ;[0.15 0.15 0.15 0.5] socket 안함
  (bind _returnvalue (Transformation|AttachComponentToComponent (Variables|/Script/Engine.Character|GetMesh _output_get) "None" "SnapToTarget" "SnapToTarget" "KeepRelative" true))
  (return _returnvalue))

(fn EventDetachfromChar
  (params (Character :type Character%20Object%20Reference))
  (Transformation|DetachFromComponent (Variables|Default|Getweapon) "KeepWorld" "KeepWorld" "KeepWorld" true)
  (Variables|Default|SetCharacter 0)
  (return false))

(fn EventTrigger
  (params (IsPressed :type Boolean))
  (if IsPressed
    (CallFunction|DoTrigger)
    (return false)))